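; BP_Banana is a banana actor that makes a noise for AI hearing when it hits something, then disappears.
; Its first Hit, gated by a DoOnce, draws a debug box around the banana mesh, plays a thump sound and reports a noise event at the mesh with itself as instigator.
; The actor destroys itself after a short delay.
; Nodes for disabling physics on the Sphere component are left disconnected.
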(event Collision|EventHit
  (params (MyComp :type Primitive%20Component%20Object%20Reference) (Other :type Actor%20Object%20Reference) (OtherComp :type Primitive%20Component%20Object%20Reference) (bSelfMoved :type Boolean) (HitLocation :type Vector :default "0, 0, 0") (HitNormal :type Vector :default "0, 0, 0") (NormalImpulse :type Vector :default "0, 0, 0") (Hit :type Hit%20Result%20Structure%20%28by%20ref%29))
  (Utilities|FlowControl|DoOnce false
    (:Completed
      (Rendering|Debug|DrawDebugBox (Transformation|GetWorldLocation (Variables|Default|GetSM_Banana)) "200.000000,200.000000,200.000000" "(R=1.000000,G=0.000000,B=0.528181,A=1.000000)" "0, 0, 0" 5.0 1e+01)
      (Audio|PlaySoundatLocation "/Game/Audio/Thump-sound-effect.Thump-sound-effect" (Transformation|GetActorLocation) "0, 0, 0" 1.0 1.0 0.0 0 0 0 0)
      (Class|AISenseHearing|ReportNoiseEvent (Transformation|GetWorldLocation (Variables|Default|GetSM_Banana)) 1.0 self 0.0 "None")
      (Utilities|FlowControl|Delay 1.0)
      (Actor|DestroyActor))))

(fn ConstructionScript)