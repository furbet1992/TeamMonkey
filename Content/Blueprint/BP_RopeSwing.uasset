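; Rope swing actor that lets the player grab, swing on, climb and leap off a cable once overlapping its box enables input.
; Holding Space attaches the player to the CableEnd socket at their current height with movement off; releasing detaches, launches them and disables input.
; WASD set directional CableForce, with no reset on release.
; E/Q climb in delayed steps between limit markers positioned by the construction script.
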(event OnComponentBeginOverlap(Box)
  (params (OverlappedComponent :type Primitive%20Component%20Object%20Reference) (OtherActor :type Actor%20Object%20Reference) (OtherComp :type Primitive%20Component%20Object%20Reference) (OtherBodyIndex :type Integer) (bFromSweep :type Boolean) (SweepResult :type Hit%20Result%20Structure%20%28by%20ref%29))
  ;[0.15 0.15 0.15 0.5] Enable Input
  (Input|EnableInput self (Game|GetPlayerController 0)))

(event Input|KeyboardEvents|SpaceBar
  (params (Key :type Key%20Structure :default "None"))
  (bind _returnvalue (Game|GetPlayerCharacter 0))
  (bind _returnvalue_2 (Transformation|GetActorLocation _returnvalue))
  (bind _charactermovement (Variables|/Script/Engine.Character|GetCharacterMovement _returnvalue))
  ;[0.15 0.15 0.15 0.5] Getting On and Off Rope
  (:Pressed
    (Variables|Default|SetPlayer%20Height (.z (Transformation|GetActorLocation (Game|GetPlayerCharacter 0))))
    (Transformation|AttachActorToActor _returnvalue (Variables|Default|GetCableREF) "CableEnd" "SnapToTarget" "KeepWorld" "KeepWorld" true)
    (Transformation|SetActorLocation _returnvalue (Math|Vector|MakeVector (.x _returnvalue_2) (.y _returnvalue_2) (Variables|Default|GetPlayer%20Height)) false false)
    (Pawn|Components|CharacterMovement|SetMovementMode _charactermovement "MOVE_None" 0))
  (:Released
    (Transformation|DetachFromActor _returnvalue "KeepWorld" "KeepWorld" "KeepWorld")
    (Pawn|Components|CharacterMovement|SetMovementMode _charactermovement "MOVE_Falling" 0)
    (Character|LaunchCharacter _returnvalue (+ (* (Transformation|GetActorForwardVector _returnvalue) 1e+03) (* (Transformation|GetActorUpVector _returnvalue) 1e+02)) false false)
    (Input|DisableInput self (Game|GetPlayerController 0))))

(event Input|KeyboardEvents|Q
  (params (Key :type Key%20Structure :default "None"))
  (bind _returnvalue (Game|GetPlayerCharacter 0))
  ;[0.15 0.15 0.15 0.5] Climb Up and Down
  (:Pressed
    (Variables|Default|SetqHeld? true)
    (if (<= (.z (Transformation|GetWorldLocation (Variables|Default|GetBottom%20Climb%20REF))) (.z (Transformation|GetActorLocation _returnvalue))) :!label _label
      (Transformation|AddActorWorldOffset _returnvalue "0.000000,0.000000,-15.000000")
      (Utilities|FlowControl|Delay 0.2)
      (if (Variables|Default|GetqHeld?)
        (goto _label))))
  (:Released
    (Variables|Default|SetqHeld? false)))

(event Input|KeyboardEvents|E
  (params (Key :type Key%20Structure :default "None"))
  (bind _returnvalue (Game|GetPlayerCharacter 0))
  ;[0.15 0.15 0.15 0.5] Climb Up and Down
  (:Pressed
    (Variables|Default|SeteHeld? true)
    (if (>= (.z (Transformation|GetWorldLocation (Variables|Default|GetTop%20Climb%20REF))) (.z (Transformation|GetActorLocation _returnvalue))) :!label _label
      (Transformation|AddActorWorldOffset _returnvalue "0.000000,0.000000,15.000000")
      (Utilities|FlowControl|Delay 0.2)
      (if (Variables|Default|GeteHeld?)
        (goto _label))))
  (:Released
    (Variables|Default|SeteHeld? false)))

(event Input|KeyboardEvents|W
  (params (Key :type Key%20Structure :default "None"))
  ;[0.15 0.15 0.15 0.5] Swing Rope
  (:Pressed
    (Variables|/Script/CableComponent.CableComponent|SetCableForce (Variables|/Script/CableComponent.CableActor|GetCableComponent (Variables|Default|GetCableREF)) "200.000000,0.000000,0.000000")))

(event Input|KeyboardEvents|S
  (params (Key :type Key%20Structure :default "None"))
  ;[0.15 0.15 0.15 0.5] Swing Rope
  (:Pressed
    (Variables|/Script/CableComponent.CableComponent|SetCableForce (Variables|/Script/CableComponent.CableActor|GetCableComponent (Variables|Default|GetCableREF)) "-200.000000,0.000000,0.000000")))

(event Input|KeyboardEvents|A
  (params (Key :type Key%20Structure :default "None"))
  ;[0.15 0.15 0.15 0.5] Swing Rope
  (:Pressed
    (Variables|/Script/CableComponent.CableComponent|SetCableForce (Variables|/Script/CableComponent.CableActor|GetCableComponent (Variables|Default|GetCableREF)) "0.000000,-200.000000,0.000000")))

(event Input|KeyboardEvents|D
  (params (Key :type Key%20Structure :default "None"))
  ;[0.15 0.15 0.15 0.5] Swing Rope
  (:Pressed
    (Variables|/Script/CableComponent.CableComponent|SetCableForce (Variables|/Script/CableComponent.CableActor|GetCableComponent (Variables|Default|GetCableREF)) "0.000000,200.000000,0.000000")))

(fn ConstructionScript
  (bind _bottom_climb_ref (Variables|Default|GetBottom%20Climb%20REF))
  (bind _top_climb_ref (Variables|Default|GetTop%20Climb%20REF))
  (bind _relativelocation (Variables|/Script/Engine.SceneComponent|GetRelativeLocation _bottom_climb_ref))
  (bind _relativelocation_2 (Variables|/Script/Engine.SceneComponent|GetRelativeLocation _top_climb_ref))
  (Transformation|SetRelativeLocation _top_climb_ref (Math|Vector|MakeVector (.x _relativelocation_2) (.y _relativelocation_2) (Variables|Default|GetTop%20Climb%20Limit)) false false)
  (Transformation|SetRelativeLocation _bottom_climb_ref (Math|Vector|MakeVector (.x _relativelocation) (.y _relativelocation) (Variables|Default|GetBottom%20Climb%20Limit)) false false))