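; AI controller for a guard that detects the player by sight.
; It starts the BT_GUARD behavior tree on BeginPlay.
; When AI Perception reports a successful sight stimulus from an actor tagged Player, it sets the hasSeenPlayer Blackboard key and prints a debug message.
; The controller never clears that key.
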(event OnTargetPerceptionUpdated(AIPerception)
  (params (Actor :type Actor%20Object%20Reference) (Stimulus :type AI%20Stimulus%20Structure))
  (bind _returnvalue (Class|AIPerceptionSystem|GetSenseClassforStimulus Stimulus))
  (if (== _returnvalue "/Script/AIModule.AISense_Sight")
    (if (and (.bSuccessfullySensed (Utilities|Struct|BreakAIStimulus Stimulus)) (Actor|ActorHasTag Actor "Player"))
      (AI|Components|Blackboard|SetValueasBool (AI|GetBlackboard 0) (Utilities|Name|MakeLiteralName "hasSeenPlayer") true)
      (Development|PrintString "Seen"))))

(event EventBeginPlay
  (AI|RunBehaviorTree "/Game/AI/BT_GUARD.BT_GUARD"))

(fn ConstructionScript)